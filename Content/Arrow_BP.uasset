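; Arrow actor that changes its orientation in response to the IA_ClickArrow input action.
; Each input increments a Counter, and a nested branch chain maps values 0 through 3 to four fixed rotations set through SetActorRotation.
; Counter never resets or wraps in this graph, so inputs that push it past 3 leave the rotation unchanged.
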(event Input|EnhancedActionEvents|EnhancedInputActionIA_ClickArrow
  (params (ActionValue :type Boolean) (ElapsedSeconds :type Float%20%28double-precision%29) (TriggeredSeconds :type Float%20%28double-precision%29) (InputAction :type Input%20Action%20Object%20Reference :default "/Game/IA_ClickArrow.IA_ClickArrow"))
  (Variables|Default|Setcounter (+ (Variables|Default|Getcounter) 1))
  (if (== (Variables|Default|Getcounter) 0)
    (Transformation|SetActorRotation "0.000000,0.000000,-90.000000")
    (elif (== (Variables|Default|Getcounter) 1)
      (Transformation|SetActorRotation "0.000000,90.000000,-90.000000")
      (elif (== (Variables|Default|Getcounter) 2)
        (Transformation|SetActorRotation "0.000000,0.000000,90.000000")
        (elif (== (Variables|Default|Getcounter) 3)
          (Transformation|SetActorRotation "0.000000,90.000000,90.000000"))))))

(event EventBeginPlay)

(event Collision|EventActorBeginOverlap
  (params (OtherActor :type Actor%20Object%20Reference)))

(event EventTick
  (params (DeltaSeconds :type Float%20%28single-precision%29)))

(fn ConstructionScript)