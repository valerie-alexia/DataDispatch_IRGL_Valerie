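; Cube_BP is a grid map tile actor with an arrow sprite whose direction is changed by clicking.
; Each click steps a Counter through four states, right, back, left and front, setting the arrow's relative rotation before wrapping around.
; A box component prints the name of any overlapping actor, and clicks also print a debug message.
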(event OnComponentBeginOverlap(Box)
  (params (OverlappedComponent :type Primitive%20Component%20Object%20Reference) (OtherActor :type Actor%20Object%20Reference) (OtherComp :type Primitive%20Component%20Object%20Reference) (OtherBodyIndex :type Integer) (bFromSweep :type Boolean) (SweepResult :type Hit%20Result%20Structure%20%28by%20ref%29))
  (Development|PrintString (Utilities|GetDisplayName OtherActor)))

(event Custom|Clicked
  (Development|PrintString "Hello")
  ;[1 1 1] Kanan 0
  (if (== (Variables|Components|Getcounter) 0)
    (Transformation|SetRelativeRotation (Variables|Default|GetArrow%20Sprite) "0.000000,0.000000,-90.000000" false false)
    (Variables|Components|Setcounter 1)
    (else
      ;[1 1 1] Back 1
      (if (== (Variables|Components|Getcounter) 1)
        (Transformation|SetRelativeRotation (Variables|Default|GetArrow%20Sprite) "0.000000,90.000000,-90.000000" false false)
        (Variables|Components|Setcounter 2)
        (else
          ;[1 1 1] Left 2
          (if (== (Variables|Components|Getcounter) 2)
            (Transformation|SetRelativeRotation (Variables|Default|GetArrow%20Sprite) "0.000000,0.000000,90.000000" false false)
            (Variables|Components|Setcounter 3)
            (else
              ;[1 1 1] Front 3
              (if (== (Variables|Components|Getcounter) 3)
                (Transformation|SetRelativeRotation (Variables|Default|GetArrow%20Sprite) "0.000000,90.000000,90.000000" false false)
                (Variables|Components|Setcounter 0)))))))))

(event EventBeginPlay)

(event Collision|EventActorBeginOverlap
  (params (OtherActor :type Actor%20Object%20Reference)))

(event EventTick
  (params (DeltaSeconds :type Float%20%28single-precision%29)))

(fn ConstructionScript)