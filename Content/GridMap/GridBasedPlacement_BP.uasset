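; Grid map actor for a frog game that teleports the Frog actor to the first ARRAYGRID position on BeginPlay.
; GenerateCube can spawn a square grid of numbered Cube_BP actors, but nothing in this graph calls it.
; A looping timer fires an empty Moving event, and the overlap handler's checks lead to no action.
; Disconnected draft logic would turn and step the frog by matching this actor's rotation to four arrow directions.
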(event Custom|Moving)

(event Custom|GenerateCube
  (bind _counter (Variables|Default|GetCounter))
  (for _index (range 0 (Variables|Default|GetMaxRows))
    (for _index_2 (range 0 (Variables|Default|GetMaxRows))
      (bind _returnvalue (Game|SpawnActorfromClass "/Game/GridMap/Cube_BP.Cube_BP_C" (Math|Transform|MakeTransform (Math|Vector|MakeVector (* _index (Variables|Default|GetActorSpacing)) (* _index_2 (Variables|Default|GetActorSpacing)) 0.0) "0, 0, 0" "1.000000,1.000000,1.000000") "Undefined" "MultiplyWithRoot" 0 0))
      (Rendering|Components|TextRender|SetText (Variables|/Game/GridMap/Cube_BP.Cube_BP_C|GetTextRender _returnvalue) (Utilities|Text|ToText(Integer) _counter))
      (Math|Integer|IncrementInt _counter))))

(event EventBeginPlay
  (bind _arraygrid_ (Variables|Default|GetARRAYGRID%20))
  (bind _output (Utilities|Array|Get(acopy) _arraygrid_))
  (bind _returnvalue (Transformation|GetWorldLocation _output))
  ;[1 1 1] SPAWN GRID MAP
  (bind _returnvalue_2 (Actor|GetActorOfClass "/Game/frog.frog_C"))
  (bind _output_get (Variables|Default|SetFrog _returnvalue_2))
  (Development|PrintString (Utilities|String|ToString(Vector) _returnvalue))
  (Transformation|SetActorLocation _output_get _returnvalue false true)
  (Utilities|Time|SetTimerbyEvent (delegate Custom|Moving) 1.0 true))

(event EventTick
  (params (DeltaSeconds :type Float%20%28single-precision%29)))

(event Collision|EventActorBeginOverlap
  (params (OtherActor :type Actor%20Object%20Reference))
  ;[1 1 1] Comment
  (for _array_element (.ARRAYGRID%20 (Variables|Default|GetARRAYGRID%20))
    (if (Actor|ActorHasTag OtherActor "None")
      (if (Utilities|Operators|EqualEqual (.rotation (Transformation|GetRelativeTransform (Variables|Transformation|GetRootComponent))) (Variables|Default|GetLeft) 0.0)
        _))))

(fn ConstructionScript)