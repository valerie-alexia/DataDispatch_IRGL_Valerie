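; GridBasedConstructed_BP is an unfinished grid-map actor meant to lay out Cube_BP actors in rows at even spacing from its location.
; The disconnected spawn loop in the event graph derives X and Y from each index's remainder and quotient by MaxRows, scaled by ActorSpacing.
; BeginPlay is empty, and the construction script only loops with an empty body beside unused position math, so nothing spawns.
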(event EventBeginPlay
  ;[1 1 1] SPAWN GRID MAP
)

(event Collision|EventActorBeginOverlap
  (params (OtherActor :type Actor%20Object%20Reference)))

(event EventTick
  (params (DeltaSeconds :type Float%20%28single-precision%29)))

(fn ConstructionScript
  (for _index (range 0 (Variables|Default|GetMaxActors))
    _))